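; Decorative-style factory crane buildable with a configurable height and a looping arm animation.
; Construction script stacks CraneFloor instances up to TopFloor and offsets CraneArm upward for each added floor.
; Tick uses delays and a DoOnce to repeatedly restart the arm animation, alternating negative and positive play rates.
; Player seat attachment and timeline-driven rotator logic are present but unwired, and OnUse is empty.
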(event EventOnUse
  (params (byCharacter :type FG%20Character%20Player%20Object%20Reference) (state :type Use%20State%20Structure%20%28by%20ref%29)))

(event EventBeginPlay
  (Components|Timeline|SetPlayRate (Variables|Default|GetTimeline_1) 0.25))

(event EventTick
  (params (DeltaSeconds :type Float%20%28single-precision%29))
  (bind _crane_arm (Variables|Default|GetCrane_Arm))
  (bind _crane_arm_2 (Variables|Default|GetCrane_Arm))
  (Utilities|FlowControl|Delay 1e+01)
  (Utilities|FlowControl|DoOnce false :!label _label
    (:Completed
      (Audio|Components|Audio|Stop _crane_arm)
      (Utilities|FlowControl|Delay 0.2)
      (Audio|Components|Audio|Play _crane_arm false)
      (Components|Timeline|SetPlayRate _crane_arm -0.4)
      (Utilities|FlowControl|Delay 1e+01)
      (Audio|Components|Audio|Stop _crane_arm_2)
      (Utilities|FlowControl|Delay 0.2)
      (Audio|Components|Audio|Play _crane_arm_2 false)
      (Components|Timeline|SetPlayRate _crane_arm_2 0.4)
      (goto _label Reset))))

(fn ConstructionScript
  (for _index (range 0 (Variables|Default|GetTopFloor))
    (if (> _index 0)
      (Utilities|FlowControl|Sequence
        (:then_0
          (Components|InstancedStaticMesh|AddInstance (Variables|Default|GetCrane_Floor) (Math|Transform|MakeTransform (Math|Vector|MakeVector 0.0 0.0 (* _index (Variables|Default|GetFloorHeight)))) :!label _label))
        (:then_1
          (Transformation|AddRelativeLocation (Variables|Default|GetCrane_Arm) (+ (Math|Vector|MakeVector 0.0 0.0 (Variables|Default|GetFloorHeight)) _index) false false)))
      (else
        (goto _label)))))