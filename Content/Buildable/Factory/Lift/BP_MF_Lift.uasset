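; BP_MF_Lift is a factory lift buildable, apparently an unfinished prototype with debug chat output.
; On BeginPlay, after a delay, it prints connection positions and stores the distance between MConnection0 and MConnection1.
; It then spawns a fixed vertical column of scaled MF_LegVertical actors at world X/Y zero, independent of that distance.
; After another short delay, it destroys both connection components.
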(event EventBeginPlay
  (bind _playercontroller (CallFunction|GetLocalController))
  (bind _mconnection0 (Variables|Default|GetmConnection0))
  (bind _mconnection1 (Variables|Default|GetmConnection1))
  (bind _returnvalue (Transformation|GetWorldTransform _mconnection0))
  (bind _returnvalue_2 (Transformation|GetWorldTransform _mconnection1))
  (bind _returnvalue_3 (Math|Vector|Distance(Vector) (.location _returnvalue) (.location _returnvalue_2)))
  (Utilities|FlowControl|Delay 1.0)
  (Class|FGPlayerController|EnterChatMessage _playercontroller "ghghghg")
  (Class|FGPlayerController|EnterChatMessage _playercontroller (Utilities|String|ToString(Float) (.z (Variables|/Script/Engine.SceneComponent|GetRelativeLocation _mconnection0))))
  (Class|FGPlayerController|EnterChatMessage _playercontroller (Utilities|String|ToString(Vector) (.location _returnvalue_2)))
  (Class|FGPlayerController|EnterChatMessage _playercontroller (Utilities|String|ToString(Float) _returnvalue_3))
  (Variables|Default|SetDistance _returnvalue_3)
  (for _index (range 0 50)
    (Game|SpawnActorfromClass "/MoarFactory/Buildable/Factory/Lift/MF_LegVertical.MF_LegVertical_C" (Math|Transform|MakeTransform (Math|Vector|MakeVector 0.0 0.0 (+ (* _index 1e+02) 4e+01)) "0, 0, 0" "1.500000,1.500000,1.500000") "Undefined" 0 0))
  (Utilities|FlowControl|Delay 0.2)
  (Components|DestroyComponent (Variables|Default|GetmConnection0)))

(fn ConstructionScript)