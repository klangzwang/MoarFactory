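; BP_BullExplorer is the Bull Explorer car Blueprint, driving cosmetic effects from direct key input, with no movement logic of its own.
; Holding W ramps wheel emissive through a timeline that reverses on release.
; Space likewise animates chassis glow and mirrored shutter rotation, activating two particle systems when the timeline finishes, while C toggles two spotlights with their chassis glow.
; Timeline updates create dynamic material instances on every tick rather than caching them.
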(event Input|KeyboardEvents|W
  (params (Key :type Key%20Structure))
  (:Pressed
    (bind _newtrack_0 (Timeline|Timeline_0 Play)
      (:Update
        (for _array_element (Utilities|Array|MakeArray (Variables|Default|Getwheel_fr) (Variables|Default|Getwheel_fl) (Variables|Default|Getwheel_br) (Variables|Default|Getwheel_bl))
          (bind _returnvalue (Rendering|Material|CreateDynamicMaterialInstance _array_element 0 0 "None" :!class /Script/Engine.PrimitiveComponent))
          (Rendering|Material|SetScalarParameterValue _returnvalue "Emissive" _newtrack_0 :!class /Script/Engine.MaterialInstanceDynamic)))))
  (:Released
    (Timeline|Timeline_0 Reverse)))

(event Input|KeyboardEvents|SpaceBar
  (params (Key :type Key%20Structure))
  (:Pressed
    (bind (_direction _newtrack_0 _newtrack_1) (Timeline|Timeline_1 Play)
      (:Update
        (bind _returnvalue (Rendering|Material|CreateDynamicMaterialInstance (Variables|Default|Getmf_vwbus_chassie) 6 0 "None" :!class /Script/Engine.PrimitiveComponent))
        (Rendering|Material|SetScalarParameterValue _returnvalue "Emissive" _newtrack_0 :!class /Script/Engine.MaterialInstanceDynamic)
        (Transformation|SetRelativeLocationAndRotation (Variables|Default|Getmf_shutterR) "76.800003,152.000000,134.000000" (Math|Rotator|MakeRotator 0.0 0.0 _newtrack_1) false false)
        (bind _result (Math|Float|NegateFloat _newtrack_1)
          (:%20%20
            (Transformation|SetRelativeLocationAndRotation (Variables|Default|Getmf_shutterL) "76.800003,-152.000000,134.000000" (Math|Rotator|MakeRotator 0.0 0.0 _result) false false))))
      (:Finished
        (Components|Activation|Activate (Variables|Default|GetParticleSystem1) false))))
  (:Released
    (Timeline|Timeline_1 Reverse)))

(event Input|KeyboardEvents|C
  (params (Key :type Key%20Structure))
  (bind _mf_vwbus_chassie (Variables|Default|Getmf_vwbus_chassie))
  (:Pressed
    (Utilities|FlowControl|FlipFlop
      (:A
        (bind _returnvalue (Rendering|Material|CreateDynamicMaterialInstance _mf_vwbus_chassie 4 0 "None" :!class /Script/Engine.PrimitiveComponent))
        (Rendering|Material|SetScalarParameterValue _returnvalue "Emissive" 2e+01 :!class /Script/Engine.MaterialInstanceDynamic)
        (Rendering|Components|Light|SetIntensity (Variables|Default|GetSpotLight_0) 5e+01))
      (:B
        (bind _returnvalue_2 (Rendering|Material|CreateDynamicMaterialInstance _mf_vwbus_chassie 4 0 "None" :!class /Script/Engine.PrimitiveComponent))
        (Rendering|Material|SetScalarParameterValue _returnvalue_2 "Emissive" 0.0 :!class /Script/Engine.MaterialInstanceDynamic)
        (Rendering|Components|Light|SetIntensity (Variables|Default|GetSpotLight_0) 0.0)))))

(fn ConstructionScript
  (|CallParentFunction))