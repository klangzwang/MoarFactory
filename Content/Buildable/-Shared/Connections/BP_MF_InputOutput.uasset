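; Animated input/output port for factory buildables that opens its doors when a conveyor belt or lift connects and closes them otherwise.
; Tick uses a Delay to throttle overlap checks on LookConveyor, then fires the open or close event.
; Cross-resetting DoOnce gates play or reverse one timeline driving doors, base parts, light, smoke and material glow, with sound cues.
; The first detection also briefly enables physics on SphereA.
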(event Custom|Event%20OpenTheHole
  (Utilities|FlowControl|Sequence
    (:then_0
      (Utilities|FlowControl|DoOnce false
        (:Completed
          (Variables|Default|SetDoorsAreOpen true)
          (Components|Activation|Activate (Variables|Default|GetDoorOpen_Cue) true)
          (bind (_direction _newtrack_0 _newtrack_1 _newtrack_2 _newtrack_4 _newtrack_5 _newtrack_6 _newtrack_7 _newtrack_8) (Timeline|Timeline_0 Play)
            (:Update
              (Transformation|SetRelativeLocation (Variables|Default|GetIOBase1-1) (Math|Vector|MakeVector _newtrack_5 0.0 0.0) false false)
              (Transformation|SetRelativeLocation (Variables|Default|GetInOutDoorL1) (Math|Vector|MakeVector _newtrack_8 (* -1 _newtrack_0) 0.0) false false)
              (Transformation|SetRelativeLocation (Variables|Default|GetInOutDoorR1) (Math|Vector|MakeVector _newtrack_8 _newtrack_0 0.0) false false)
              (Rendering|Components|Light|SetIntensity (Variables|Default|GetLight0) _newtrack_2)
              (CallFunction|CalcInputColorIntensity _newtrack_4)
              (Transformation|SetRelativeLocation (Variables|Default|GetIOBase2-1) (Math|Vector|MakeVector _newtrack_7 0.0 0.0) false false))
            (:NewTrack_3
              (Components|Activation|Activate (Variables|Default|GetSmoke0) false))))))
    (:then_1
      (Utilities|FlowControl|DoOnce true) ; enters at Reset
    )))

(event Custom|Event%20CloseTheHole
  (Utilities|FlowControl|Sequence
    (:then_0
      (Utilities|FlowControl|DoOnce true
        (:Completed
          (Variables|Default|SetDoorsAreOpen false)
          (Components|Activation|Activate (Variables|Default|GetDoorClose_Cue) true)
          (bind (_direction _newtrack_0 _newtrack_1 _newtrack_2 _newtrack_4 _newtrack_5 _newtrack_6 _newtrack_7 _newtrack_8) (Timeline|Timeline_0 Reverse)
            (:Update
              (Transformation|SetRelativeLocation (Variables|Default|GetIOBase1-1) (Math|Vector|MakeVector _newtrack_5 0.0 0.0) false false)
              (Transformation|SetRelativeLocation (Variables|Default|GetInOutDoorL1) (Math|Vector|MakeVector _newtrack_8 (* -1 _newtrack_0) 0.0) false false)
              (Transformation|SetRelativeLocation (Variables|Default|GetInOutDoorR1) (Math|Vector|MakeVector _newtrack_8 _newtrack_0 0.0) false false)
              (Rendering|Components|Light|SetIntensity (Variables|Default|GetLight0) _newtrack_2)
              (CallFunction|CalcInputColorIntensity _newtrack_4)
              (Transformation|SetRelativeLocation (Variables|Default|GetIOBase2-1) (Math|Vector|MakeVector _newtrack_7 0.0 0.0) false false))
            (:NewTrack_3
              (Components|Activation|Activate (Variables|Default|GetSmoke0) false))))))
    (:then_1
      (Utilities|FlowControl|DoOnce false) ; enters at Reset
    )))

(event EventTick
  (params (DeltaSeconds :type Float%20%28single-precision%29))
  (Utilities|FlowControl|Delay 0.2)
  (bind _conveyorliftconnected (CallFunction|LookforLift))
  (bind _conveyorconnected (CallFunction|LookforBelt))
  (if (or _conveyorconnected _conveyorliftconnected)
    (CallFunction|EventOpentheHole)
    (Utilities|FlowControl|DoOnce false
      (:Completed
        (Utilities|FlowControl|Delay 0.5)
        (Physics|SetSimulatePhysics (Variables|Default|GetSphereA) true)
        (Utilities|FlowControl|Delay 4.0)
        (Physics|SetSimulatePhysics (Variables|Default|GetSphereA) false)))
    (else
      (CallFunction|EventClosetheHole))))

(event EventBeginPlay
  (CallFunction|CalcInputColorIntensity 0.0))

(fn ConstructionScript)

(fn CalcInputColorIntensity
  (params (Value :type Float%20%28single-precision%29))
  (for _array_element (Utilities|Array|MakeArray 0 0)
    (bind _returnvalue (Rendering|Material|CreateDynamicMaterialInstance _array_element 0 "/Game/FactoryGame/-Shared/Material/MI_Factory_Base_01.MI_Factory_Base_01" "None" :!class /Script/Engine.PrimitiveComponent))
    (Rendering|Material|SetScalarParameterValue _returnvalue "InputColorIntensity" Value :!class /Script/Engine.MaterialInstanceDynamic)))

(fn LookforBelt
  (bind _returnvalue (Collision|ComponentOverlapActors (Variables|Default|GetLookConveyor) (Transformation|GetActorTransform self) (Utilities|Array|MakeArray "ObjectTypeQuery2" "ObjectTypeQuery1") "/Script/FactoryGame.FGBuildableConveyorBelt" (Utilities|Array|MakeArray self)))
  (return _returnvalue))

(fn LookforLift
  (bind _returnvalue (Collision|ComponentOverlapActors (Variables|Default|GetLookConveyor) (Transformation|GetActorTransform self) (Utilities|Array|MakeArray "ObjectTypeQuery2" "ObjectTypeQuery1") "/Script/FactoryGame.FGBuildableConveyorLift" (Utilities|Array|MakeArray self)))
  (return _returnvalue))