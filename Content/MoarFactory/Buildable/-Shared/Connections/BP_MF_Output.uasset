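; Animated output port for MoarFactory buildables that opens its doors when a conveyor belt or lift is attached.
; Tick, throttled by a Delay, runs component overlap checks for belts and lifts to choose open or close.
; Paired DoOnce gates reset each other so sound cues and timeline play or reverse only on state changes.
; The timeline moves doors and parts, triggers smoke, and drives light and glow intensity through dynamic materials.
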(event Custom|Event%20OpenTheHole
  (Utilities|FlowControl|Sequence
    (:then_0
      (Utilities|FlowControl|DoOnce false
        (:Completed
          (Components|Activation|Activate (Variables|Default|GetDoorOpen_Cue) true)
          (bind (_direction _newtrack_0 _newtrack_1 _newtrack_2 _newtrack_4 _newtrack_5 _newtrack_6 _newtrack_7) (Timeline|Timeline_0 Play)
            (:Update
              (Transformation|SetRelativeLocation (Variables|Default|GetIOBase1) (Math|Vector|MakeVector _newtrack_5 0.0 0.0) false false)
              (Transformation|SetRelativeLocation (Variables|Default|GetDoorL) (Math|Vector|MakeVector (* -1 _newtrack_0) _newtrack_1 0.0) false false)
              (Transformation|SetRelativeLocation (Variables|Default|GetDoorR) (Math|Vector|MakeVector _newtrack_0 _newtrack_1 0.0) false false)
              (Rendering|Components|Light|SetIntensity (Variables|Default|GetLight) _newtrack_2)
              (CallFunction|CalcInputColorIntensity _newtrack_4)
              (Transformation|SetRelativeRotation (Variables|Default|GetInput_part1) (Math|Rotator|MakeRotator _newtrack_6 0.0 0.0) false false)
              (Transformation|SetRelativeLocation (Variables|Default|GetIOBase2) (Math|Vector|MakeVector 0.0 _newtrack_7 0.0) false false))
            (:NewTrack_3
              (Components|Activation|Activate (Variables|Default|GetSmoke) false))))))
    (:then_1
      (Utilities|FlowControl|DoOnce false) ; enters at Reset
    )))

(event Custom|Event%20CloseTheHole
  (Utilities|FlowControl|Sequence
    (:then_0
      (Utilities|FlowControl|DoOnce false
        (:Completed
          (Components|Activation|Activate (Variables|Default|GetDoorClose_Cue) true)
          (bind (_direction _newtrack_0 _newtrack_1 _newtrack_2 _newtrack_4 _newtrack_5 _newtrack_6 _newtrack_7) (Timeline|Timeline_0 Reverse)
            (:Update
              (Transformation|SetRelativeLocation (Variables|Default|GetIOBase1) (Math|Vector|MakeVector _newtrack_5 0.0 0.0) false false)
              (Transformation|SetRelativeLocation (Variables|Default|GetDoorL) (Math|Vector|MakeVector (* -1 _newtrack_0) _newtrack_1 0.0) false false)
              (Transformation|SetRelativeLocation (Variables|Default|GetDoorR) (Math|Vector|MakeVector _newtrack_0 _newtrack_1 0.0) false false)
              (Rendering|Components|Light|SetIntensity (Variables|Default|GetLight) _newtrack_2)
              (CallFunction|CalcInputColorIntensity _newtrack_4)
              (Transformation|SetRelativeRotation (Variables|Default|GetInput_part1) (Math|Rotator|MakeRotator _newtrack_6 0.0 0.0) false false)
              (Transformation|SetRelativeLocation (Variables|Default|GetIOBase2) (Math|Vector|MakeVector 0.0 _newtrack_7 0.0) false false))
            (:NewTrack_3
              (Components|Activation|Activate (Variables|Default|GetSmoke) false))))))
    (:then_1
      (Utilities|FlowControl|DoOnce false) ; enters at Reset
    )))

(event EventTick
  (params (DeltaSeconds :type Float%20%28single-precision%29))
  (Utilities|FlowControl|Delay 0.2)
  (bind _conveyorconnected (CallFunction|LookforLift))
  (bind _conveyorconnected_2 (CallFunction|LookforBelt))
  (if (or _conveyorconnected_2 _conveyorconnected)
    (CallFunction|EventOpentheHole)
    (else
      (CallFunction|EventClosetheHole))))

(event EventBeginPlay
  (CallFunction|CalcInputColorIntensity 0.0))

(fn ConstructionScript)

(fn CalcInputColorIntensity
  (params (Value :type Float%20%28single-precision%29))
  (for _array_element (Utilities|Array|MakeArray (Variables|Default|GetInput_part1) (Variables|Default|GetInput_part2) (Variables|Default|GetInput_part3) (Variables|Default|GetDoorR) (Variables|Default|GetDoorL))
    (bind _returnvalue (Rendering|Material|CreateDynamicMaterialInstance _array_element 0 "/Game/FactoryGame/-Shared/Material/MI_Factory_Base_01.MI_Factory_Base_01" "None" :!class /Script/Engine.PrimitiveComponent))
    (Rendering|Material|SetScalarParameterValue _returnvalue "InputColorIntensity" Value :!class /Script/Engine.MaterialInstanceDynamic)))

(fn LookforBelt
  (bind _returnvalue (Collision|ComponentOverlapActors (Variables|Default|GetLookConveyor) (Transformation|GetActorTransform self) (Utilities|Array|MakeArray "ObjectTypeQuery2" "ObjectTypeQuery1") "/Script/FactoryGame.FGBuildableConveyorBelt" (Utilities|Array|MakeArray self)))
  (return _returnvalue))

(fn LookforLift
  (bind _returnvalue (Collision|ComponentOverlapActors (Variables|Default|GetLookConveyor) (Transformation|GetActorTransform self) (Utilities|Array|MakeArray "ObjectTypeQuery2" "ObjectTypeQuery1") "/Script/FactoryGame.FGBuildableConveyorLift" (Utilities|Array|MakeArray self)))
  (return _returnvalue))